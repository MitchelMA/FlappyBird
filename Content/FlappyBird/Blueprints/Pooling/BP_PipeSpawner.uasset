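; BP_PipeSpawner spawns Flappy Bird pipe obstacles from the ObstaclePool as the player progresses.
; On BeginPlay it finds the BirdCharacter and binds to its started and passed-obstacle delegates.
; Each event requests one pipe through SpawnPipe, then randomizes its gap height and height offset within configured ranges.
; BeginPlay also prints the root of a test formula, unrelated to spawning.
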(event `self.ReceiveBeginPlay`
  ;[1 1 1] When the player first gives input and every time they pass an obstacle, request a pipe from the ObstaclePool
  (`KismetSystemLibrary.PrintString` (`KismetStringLibrary.Conv_Vector2dToString` (`BPL_LinearFormula.GetRoot` (`BPL_LinearFormula.CreateFormula` 0.1 1.0))))
  (bind _returnvalue (`GameplayStatics.GetActorOfClass` "/Script/FlappyBird.BirdCharacter"))
  (add `BirdCharacter.OnBirdStartedDelegate` _returnvalue (delegate `BirdStarted`))
  (add `BirdCharacter.OnBirdPassedObstacleDelegate` _returnvalue (delegate `BirdPassed`)))

(event `BirdPassed`
  (bind (_x _y) (`KismetMathLibrary.BreakVector2D` (`self.OpeningHeights`)))
  (bind (_x_2 _y_2) (`KismetMathLibrary.BreakVector2D` (`self.Offsets`)))
  ;[1 1 1] When the player first gives input and every time they pass an obstacle, request a pipe from the ObstaclePool
  (bind _returnvalue (`self.SpawnPipe` :!label _label))
  (`PipeObstacle.SetGapHeight` _returnvalue (`KismetMathLibrary.RandomFloatInRange` _x _y))
  (`PipeObstacle.SetHeightOffset` _returnvalue (`KismetMathLibrary.RandomFloatInRange` _x_2 _y_2)))

(event `BirdStarted`
  ;[1 1 1] When the player first gives input and every time they pass an obstacle, request a pipe from the ObstaclePool
  (goto _label))

(fn `UserConstructionScript`)