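; Flappy Bird pipe spawner that starts spawning when the bird's start delegate fires.
; An overlap on SpawnTrigger passes a DoOnce, re-armed on end overlap, then waits SpawnDelay and spawns the next pipe unless the bird is dead.
; Each triggered spawn adds DelayAddition to SpawnDelay, so the wait grows as the run continues.
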(event `self.ReceiveBeginPlay`
  (bind _returnvalue (`GameplayStatics.GetActorOfClass` "/Script/FlappyBird.BirdCharacter"))
  (add `BirdCharacter.OnBirdStartedDelegate` _returnvalue (delegate `BirdStarted`)))

(event `BirdStarted`
  (`self.SpawnPipe`))

(event `self.SpawnTrigger.OnComponentEndOverlap`
  (params (OverlappedComponent :type "PrimitiveComponent Object Reference") (OtherActor :type "Actor Object Reference") (OtherComp :type "PrimitiveComponent Object Reference") (OtherBodyIndex :type Integer))
  (bind _spawndelay (`self.SpawnDelay`))
  (goto _label :!via `Reset`))

(event `self.SpawnTrigger.OnComponentBeginOverlap`
  (params (OverlappedComponent :type "PrimitiveComponent Object Reference") (OtherActor :type "Actor Object Reference") (OtherComp :type "PrimitiveComponent Object Reference") (OtherBodyIndex :type Integer) (bFromSweep :type Boolean) (SweepResult :type "HitResult Structure (by ref)"))
  (bind _spawndelay (`self.SpawnDelay`))
  (`/Engine/EditorBlueprintResources/StandardMacros.DoOnce` false :!label _label
    (:`Completed`
      (`KismetSystemLibrary.PrintString` (`KismetSystemLibrary.GetDisplayName` OtherActor) true true (struct :`R` 1.0 :`G` 0.084288 :`A` 1.0))
      (`KismetSystemLibrary.Delay` _spawndelay)
      (bind _returnvalue (`GameplayStatics.GetActorOfClass` "/Script/FlappyBird.BirdCharacter"))
      (if (not (`BirdCharacter.bIsBirdDead` _returnvalue))
        (set `self.SpawnDelay` (+ _spawndelay (`self.DelayAddition`)))
        (`self.SpawnPipe`)))))

(fn `UserConstructionScript`)