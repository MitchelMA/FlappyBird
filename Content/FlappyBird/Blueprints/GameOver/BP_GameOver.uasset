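; Game over actor for multiplayer Flappy Bird that shows the end screen once all players have died.
; It binds to the game state's all-players-died event on BeginPlay.
; On game over it creates either a server or client widget based on IsServer, fills in score and high score from ScoreCounter, adds it to the viewport and calls Open.
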(event `self.ReceiveBeginPlay`
  ;[1 1 1] Listen to when all the players died
  (bind _asflappy_bird_game_state (cast `FlappyBirdGameState` (`GameplayStatics.GetGameState`)))
  (bind _output_get (set `self.GameState` _asflappy_bird_game_state))
  (add `FlappyBirdGameState.OnAllPlayersDiedEvent` _output_get (delegate `AllPlayersDied`)))

(event `AllPlayersDied`
  ;[1 1 1] Listen to when all the players died
  (`self.OnGameOver`))

(event `OnGameOver`
  ;[1 1 1] Show the game over screen for the server/client
  (if (`KismetSystemLibrary.IsServer`)
    (bind _returnvalue (`|CreateWidget` (`self.ServerWidget`) (`GameplayStatics.GetPlayerControllerFromID` 0)))
    (`self.SetScore` _returnvalue)
    (`UserWidget.AddToViewport` _returnvalue 0)
    (else
      (bind _returnvalue_2 (`|CreateWidget` (`self.ClientWidget`) (`GameplayStatics.GetPlayerControllerFromID` 0)))
      (`self.SetScore` _returnvalue_2)
      (`UserWidget.AddToViewport` _returnvalue_2 0)))
  (`self.Open`))

(event `SetScore`
  (params (Widget :type "UserWidget Object Reference"))
  (bind _scorecounter (`self.ScoreCounter`))
  ;[1 1 1] Sets the display score and the high-score of the widget
  (message `GameOverWidget.SetWidgetDisplayScore` Widget (`ScoreCounter.Score` _scorecounter))
  (message `GameOverWidget.SetWidgetDisplayHighScore` Widget (`/Game/FlappyBird/Blueprints/BP_ScoreCounter.HighScore` _scorecounter)))

(fn `UserConstructionScript`)