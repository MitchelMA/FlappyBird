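; BP_BirdCharacter is the Flappy Bird character Blueprint that adds sound feedback to the bird's gameplay events.
; On BeginPlay it binds to the flap, passed-obstacle, hit-obstacle and death delegates, and each handler plays its own 2D sound.
; A boolean guard limits the hit sound to the first obstacle collision.
; The graph holds no movement or collision logic, and the construction script is empty.
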(event `self.ReceiveBeginPlay`
  ;[1 1 1] Play sounds to the corresponding events
  (add `self.OnBirdFlapped` (delegate `OnBirdFlapDelegate_Event`))
  (add `self.OnBirdPassedObstacle` (delegate `OnBirdPassedObstacleDelegate_Event`))
  (add `self.OnBirdHitObstacle` (delegate `OnBirdHitObstacleDelegate_Event`))
  (add `self.OnBirdDied` (delegate `OnBirdDiedDelegate_Event`)))

(event `OnBirdDiedDelegate_Event`
  ;[1 1 1] Play sounds to the corresponding events
  (`GameplayStatics.PlaySound2D` (`self.DeathSound`) 1.0 1.0 0.0 null null))

(event `OnBirdFlapDelegate_Event`
  ;[1 1 1] Play sounds to the corresponding events
  (`GameplayStatics.PlaySound2D` (`self.FlapSound`) 1.0 1.0 0.0 null null))

(event `OnBirdPassedObstacleDelegate_Event`
  ;[1 1 1] Play sounds to the corresponding events
  (`GameplayStatics.PlaySound2D` (`self.PointSound`) 1.0 1.0 0.0 null null))

(event `OnBirdHitObstacleDelegate_Event`
  ;[1 1 1] Play sounds to the corresponding events
  (if (not (`self.HasAlreadyHitObstacle`))
    (set `self.HasAlreadyHitObstacle` true)
    (`GameplayStatics.PlaySound2D` (`self.HitSound`) 1.0 1.0 0.0 null null)))

(fn `UserConstructionScript`)