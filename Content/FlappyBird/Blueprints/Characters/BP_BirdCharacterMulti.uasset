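; Multiplayer Flappy Bird character that lets a dead bird drift backward while other players are still alive.
; Its own death sets the speed component's disabled flag to the all-dead state, so drifting runs only if others survive.
; Tick offsets the actor along negative X at the component's speed while that flag is off.
; The game state's all-players-died event disables the speed, halting the movement.
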(event `self.ReceiveBeginPlay`
  ;[1 1 1] Get a reference to the game state
  (bind _asflappy_bird_game_state (cast `FlappyBirdGameState` (`GameplayStatics.GetGameState`)))
  (set `self.GameState` _asflappy_bird_game_state)
  (`parent.ReceiveBeginPlay`)
  ;[1 1 1] Listen to when the bird itself died
  (add `BirdCharacter.OnBirdDied` (delegate `SelfDied`))
  ;[1 1 1] Listen to when all the players on the game died
  (add `FlappyBirdGameState.OnAllPlayersDiedEvent` (`self.GameState`) (delegate `AllPlayersDied`)))

(event `SelfDied`
  ;[1 1 1] Listen to when the bird itself died
  (`SpeedComponent.SetIsSpeedDisabled` (`self.ScoreSpeedComponents`) (`self.AllDead`)))

(event `AllPlayersDied`
  ;[1 1 1] Listen to when all the players on the game died
  (`SpeedComponent.SetIsSpeedDisabled` (`self.ScoreSpeedComponents`) true)
  (set `self.AllDead` true))

(event `self.ReceiveTick`
  (params (DeltaSeconds :type "Float (single-precision)"))
  (bind _scorespeedcomponents (`self.ScoreSpeedComponents`))
  ;[1 1 1] Moves the dead bird at the speed of the component
  (`parent.ReceiveTick` DeltaSeconds)
  (if (not (`SpeedComponent.bIsSpeedDisabled` _scorespeedcomponents))
    (`self.K2_AddActorWorldOffset` (`KismetMathLibrary.MakeVector` (* (`SpeedComponent.GetSpeed` _scorespeedcomponents) DeltaSeconds -1.0)))))

(fn `UserConstructionScript`
  (`parent.UserConstructionScript`))